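; Main menu prop actor that spins its platform and lets the player set off explosions by clicking.
; Tick adds a small fixed relative rotation to the Platform component each frame, without scaling by delta time.
; The MainMenuExplosionClick input deprojects the mouse into the world and traces along that ray on the Visibility channel.
; It spawns BP_Explosion at the hit location, without checking whether the trace hit anything.
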(event `self.ReceiveTick`
  (params (DeltaSeconds :type "Float (single-precision)"))
  (`SceneComponent.K2_AddRelativeRotation` (`self.Platform`) (struct :`Yaw` 0.3) false false))

(event `InputAction|MainMenuExplosionClick`
  (params (Key :type "Key Structure"))
  (bind (_worldlocation _worlddirection _returnvalue) (`PlayerController.DeprojectMousePositionToWorld` (`GameplayStatics.GetPlayerController` 0)))
  (:`Pressed`
    (if _returnvalue
      (bind _outhit (`KismetSystemLibrary.LineTraceSingle` :`Start` _worldlocation :`End` (+ _worldlocation (* _worlddirection 2000.0)) :`TraceChannel` "TraceTypeQuery1" :`bIgnoreSelf` false))
      (`|SpawnActorFromClass` "/Game/Blueprints/Props/MainMenu/BP_Explosion.BP_Explosion_C" (`KismetMathLibrary.MakeTransform` (`.Location` (`GameplayStatics.BreakHitResult` _outhit))) "AlwaysSpawn" "OverrideRootScale" null null))))

(fn `UserConstructionScript`)