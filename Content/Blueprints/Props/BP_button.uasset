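; Pressure button prop that charges a powerline while enough actors of the allowed kind overlap its trigger.
; The construction script uses Access (Both, Jax, Leggers) to set the class filter, overlap threshold and button material.
; Tick polls the trigger, toggles green emissive and the charging flag, and passes that flag to the powerline.
; Release moves the button to its start position, but the press-down move is disconnected.
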(event `self.ReceiveTick`
  (params (DeltaSeconds :type "Float (single-precision)"))
  (if (> (`KismetArrayLibrary.Array_Length` (`PrimitiveComponent.GetOverlappingActors` (`self.ButtonTrigger`) (`self.ClassReference`))) (`self.OverlappingActorStart`))
    (`self.LowerButton`)
    (else
      (`self.ElevateButton`)))
  (`/Game/Blueprints/Components/PowerlineComponent.ChargePowerline` (`self.PowerlineComponent1`) (`self.pwrIsCharging`)))

(event `LowerButton`
  (set `self.pwrIsCharging` true)
  (`MeshComponent.SetVectorParameterValueOnMaterials` (`self.ButtonBase`) "EmissiveColor" (0.0 0.8 0.0)))

(event `ElevateButton`
  (set `self.pwrIsCharging` false)
  (`MeshComponent.SetVectorParameterValueOnMaterials` (`self.ButtonBase`) "EmissiveColor" (0.0 0.0 0.0))
  (`KismetSystemLibrary.MoveComponentTo` null (`self.Button_Start`) (struct) false false 0.1))

(fn `getActiveStatus`
  (returns (IsActive :type Boolean))
  (return (`self.IsActive`)))

(fn `setActiveStatus`
  (params (isActive :type Boolean))
  (returns (isActiveOut :type Boolean))
  (bind _output_get (set `self.IsActive` isActive))
  (return _output_get))

(fn `UserConstructionScript`
  (bind _buttonbase (`self.ButtonBase`))
  (switch `/Game/Blueprints/Props/Enums/AccessEnum` (`self.Access`)
    (:`NewEnumerator0`
      (set `self.ClassReference` null)
      (`PrimitiveComponent.SetMaterial` _buttonbase 0 "/Game/JandL_Models/NormalButton/universal/Blue.Blue")
      (set `self.OverlappingActorStart` 1))
    (:`NewEnumerator1`
      (set `self.ClassReference` "/Game/Blueprints/Characters/Jax.Jax_C")
      (`PrimitiveComponent.SetMaterial` _buttonbase 0 "/Game/JandL_Models/NormalButton/JaxButton/Hand.Hand")
      (set `self.OverlappingActorStart` 0 :!label _label))
    (:`NewEnumerator2`
      (set `self.ClassReference` "/Game/Blueprints/Characters/Leggers.Leggers_C")
      (`PrimitiveComponent.SetMaterial` _buttonbase 0 "/Game/JandL_Models/NormalButton/LeggersButton/Foot.Foot")
      (goto _label))))