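; Timed button prop that sinks when lowered and rises back over its activation time, usable by Jax, Leggers or both.
; The construction script uses Access to set the allowed class, button material and starting overlap count.
; LowerButton turns the emissive green and flags power as charging.
; ElevateButton uses a DoOnce to raise the button while active and clear both, resetting the gate when called inactive.
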(event `self.ReceiveBeginPlay`
  (set `self.Button_End` (0.0 0.0 -10.0))
  (set `self.Button_Start` (`SceneComponent.RelativeLocation` (`self.Button`))))

(event `self.LowerButton`
  (set `self.pwrIsCharging` true)
  (`MeshComponent.SetVectorParameterValueOnMaterials` (`self.Button`) "EmissiveColor" (0.0 0.8 0.0))
  (`KismetSystemLibrary.MoveComponentTo` (`self.Button`) (`self.Button_End`) (struct) false false 0.1))

(event `self.ElevateButton`
  (if (`self.IsActive`)
    (`/Engine/EditorBlueprintResources/StandardMacros.DoOnce` false :!label _label
      (:`Completed`
        (`KismetSystemLibrary.MoveComponentTo` (`self.Button`) (`self.Button_Start`) (struct) false false (`self.ActivationTime`))
        (set `self.pwrIsCharging` false)
        (`MeshComponent.SetVectorParameterValueOnMaterials` (`self.Button`) "EmissiveColor" (0.0 0.0 0.0))))
    (else
      (goto _label :!via `Reset`))))

(fn `UserConstructionScript`
  (bind _button (`self.Button`))
  (switch `/Game/Blueprints/Props/Enums/AccessEnum` (`self.Access`)
    (:`NewEnumerator0`
      (set `self.ClassReference` null)
      (`PrimitiveComponent.SetMaterial` _button 0 "/Game/Textures/Buttons/Red.Red")
      (set `self.OverlappingActorStart` 1))
    (:`NewEnumerator1`
      (set `self.ClassReference` "/Game/Blueprints/Characters/Jax.Jax_C")
      (`PrimitiveComponent.SetMaterial` _button 0 "/Game/Blueprints/Materials/M_TimedButton_Jax.M_TimedButton_Jax")
      (set `self.OverlappingActorStart` 0 :!label _label))
    (:`NewEnumerator2`
      (set `self.ClassReference` "/Game/Blueprints/Characters/Leggers.Leggers_C")
      (`PrimitiveComponent.SetMaterial` _button 0 "/Game/Blueprints/Materials/M_TimedButton_Leggers.M_TimedButton_Leggers")
      (goto _label))))