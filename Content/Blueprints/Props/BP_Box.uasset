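; BP_Box is a physics box prop that can follow a given actor, hovering in front of it.
; FollowTarget stores or clears the target and zeroes the cube's linear velocity in both cases.
; While a target is valid, Tick interpolates the box toward a point ahead of it and turns it to face the target.
; GetHoverComponent exposes its hover component, while Pull is a stub returning a zero vector.
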(event `/Game/Blueprints/Interfaces/BPI_Block.FollowTarget`
  (params (ActorToFollow :type "Actor Object Reference"))
  (if (`KismetSystemLibrary.IsValid` ActorToFollow)
    (set `self.TargetToFollow` ActorToFollow)
    (else
      (set `self.TargetToFollow` null)))
  (`PrimitiveComponent.SetAllPhysicsLinearVelocity` (`self.Cube`) (0.0 0.0 0.0) false))

(event `self.ReceiveTick`
  (params (DeltaSeconds :type "Float (single-precision)"))
  (bind _targettofollow (`self.TargetToFollow`)
    (:`then`
      (bind _returnvalue (`self.K2_GetActorLocation` _targettofollow))
      (`self.K2_SetActorLocationAndRotation` (`KismetMathLibrary.VInterpTo` (`self.K2_GetActorLocation`) (+ (* (`self.GetActorForwardVector` _targettofollow) (`self.FollowDistance`)) _returnvalue) DeltaSeconds (`self.FollowSpeed`)) (`KismetMathLibrary.FindLookAtRotation` (`self.K2_GetActorLocation`) _returnvalue)))
    (:`else`)))

(fn `GetHoverComponent`
  (returns (HoverComp :type "/Game/Blueprints/Components/HoverComponent Object Reference"))
  (return (`self.HoverComponent`)))

(fn `Pull`
  (params (Location :type "Vector Structure"))
  (returns (LocationOut :type "Vector Structure"))
  (return (0.0 0.0 0.0)))

(fn `UserConstructionScript`)