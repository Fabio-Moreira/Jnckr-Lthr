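; Puzzle-style prism prop that emits a beam while both its left and right actor inputs are set.
; Each tick it line-traces from BeamOutput, ignoring Glass-tagged actors, and creates or updates a PrismBeam, destroying it when input is lost.
; Teleport mode cycles positions of both inputs and a magnetic target in either direction.
; Signal mode toggles Green/Orange-tagged receivers, while Magnet mode drives the target's HoverComponent, both gated by SignalDone.
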(event `self.ReceiveBeginPlay`
  (bind _outactors (`GameplayStatics.GetAllActorsWithTag` "Glass"))
  (set `self.GlassToIgnore` _outactors))

(event `self.ReceiveTick`
  (params (DeltaSeconds :type "Float (single-precision)"))
  (`parent.ReceiveTick` DeltaSeconds)
  (bind _hasplayerinput (`self.HasPlayerInput`))
  (if _hasplayerinput
    (`self.CheckLine`)
    (`self.BeamTick`)
    (else
      ;[1 1 1] If there is a beam but no longer a player input the beam will be destroyed
      (`/Engine/EditorBlueprintResources/StandardMacros.IsValid` (`self.PrismBeam`)
        (:`Is Valid`
          (`self.DestroyBeam`))))))

(event `ClearActors`
  (set `self.LeftActor` null)
  (set `self.RightActor` null)
  (set `self.ResetSignalBeam` true))

(event `UsePrism`
  (params (BeamType :type "/Game/Blueprints/Beams/Enum_BeamType Enum" :default "NewEnumerator0"))
  (set `self.Enum_BeamType` BeamType))

(event `OptionOne`
  (switch `/Game/Blueprints/Beams/Enum_BeamType` (`self.Enum_BeamType`)
    (:`NewEnumerator2`
      (`self.LeftToRight`))))

(event `OptionTwo`
  (switch `/Game/Blueprints/Beams/Enum_BeamType` (`self.Enum_BeamType`)
    (:`NewEnumerator2`
      (`self.RightToLeft`))))

(event `CustomEvent`)

(fn `BeamTick`
  (bind _enum_beamtype (`self.Enum_BeamType`))
  ;[1 1 1] Check if there is already an existing beam
  (`/Engine/EditorBlueprintResources/StandardMacros.IsValid` (`self.PrismBeam`)
    (:`Is Valid`
      (`self.UpdateLocationValues`)
      ;[1 1 1] Check if the beam has been changed since the last tick and if so it will change the beam color
      (if (!= (`/Game/Blueprints/Beams/PrismBeams/PrismBeam.Enum_BeamType` (`self.PrismBeam`)) (`self.Enum_BeamType`))
        (`/Game/Blueprints/Beams/PrismBeams/PrismBeam.UpdateBeamType` (`self.PrismBeam`) _enum_beamtype)
        (else
          (switch `/Game/Blueprints/Beams/Enum_BeamType` _enum_beamtype
            (:`NewEnumerator0`
              (if (not (`self.SignalDone`))
                (`self.SignalBeam`)))
            (:`NewEnumerator1`
              (if (not (`self.SignalDone`))
                (`self.MagnetBeam`)))))))
    (:`Is Not Valid`
      ;[1 1 1] Creates a beam / updates the location values for the beam / updates the beam type to change the color to the selected beam color
      (`self.CreateBeam`)
      (`self.UpdateLocationValues`)
      (`/Game/Blueprints/Beams/PrismBeams/PrismBeam.UpdateBeamType` (`self.PrismBeam`) (`self.Enum_BeamType`)))))

(fn `CheckLine`
  ;[1 1 1] Throws a line from the BeamOutput scene component and stores the actor hit by the line and the location it has hit an actor / Always hits something even if it is only a wall
  (bind _outhit (`KismetSystemLibrary.LineTraceSingle` (`SceneComponent.K2_GetComponentLocation` (`self.BeamOutput`)) (`KismetMathLibrary.GreaterGreater_VectorRotator` (50000.0 0.0 0.0) (`self.K2_GetActorRotation`)) "TraceTypeQuery1" false (`self.GlassToIgnore`)))
  (set `self.LineHitLocation` (`.Location` (`GameplayStatics.BreakHitResult` _outhit)))
  (set `self.LineHitActor` (`.HitActor` (`GameplayStatics.BreakHitResult` _outhit)))
  (return))

(fn `CreateBeam`
  (locals (BeamTransform :type "Transform Structure"))
  (bind _returnvalue (`|SpawnActorFromClass` "/Game/Blueprints/Beams/PrismBeams/PrismBeam.PrismBeam_C" (`KismetMathLibrary.Conv_VectorToTransform` (0.0 0.0 0.0)) "Undefined" "OverrideRootScale" null null))
  (bind _output_get (set `self.PrismBeam` _returnvalue))
  (set `/Game/Blueprints/Beams/PrismBeams/PrismBeam.Enum_BeamType` (`self.Enum_BeamType`) _output_get))

(fn `DestroyBeam`
  (`self.K2_DestroyActor` (`self.PrismBeam`)))

(fn `HasPlayerInput`
  (returns (HasPlayerInput :type Boolean))
  (return (and (`KismetSystemLibrary.IsValid` (`self.LeftActor`)) (`KismetSystemLibrary.IsValid` (`self.RightActor`)))))

(fn `LeftToRight`
  (locals (LOutputlocation :type "Vector Structure" :default (0.0 0.0 0.0)) (LLeftActorLocation :type "Vector Structure" :default (0.0 0.0 0.0)) (LRightActorLocation :type "Vector Structure" :default (0.0 0.0 0.0)))
  (bind _valid (`self.VerifyLeftRight`))
  (if _valid
    (if (`KismetSystemLibrary.DoesImplementInterface` (`self.LineHitActor`) "/Game/Blueprints/Interfaces/BPI_Magnetic.BPI_Magnetic_C")
      (set `local.LLeftActorLocation` (`self.K2_GetActorLocation` (`self.LeftActor`)))
      (set `local.LRightActorLocation` (`self.K2_GetActorLocation` (`self.RightActor`)))
      (bind _output_get (set `local.LOutputlocation` (`self.LineHitLocation`)))
      (`self.K2_TeleportTo` :`self` (`self.LeftActor`) :`DestLocation` _output_get)
      (`self.K2_TeleportTo` :`self` (`self.RightActor`) :`DestLocation` (`local.LLeftActorLocation`))
      (`self.K2_TeleportTo` :`self` (`self.LineHitActor`) :`DestLocation` (`local.LRightActorLocation`))
      (`self.DestroyBeam`))))

(fn `MagnetBeam`
  (locals (Speed :type "Vector Structure" :default (5.0 5.0 0.0)) (Pushed :type Boolean) (Pulled :type Boolean))
  (bind _linehitactor (`self.LineHitActor`))
  (bind _returnvalue (`self.GetComponentByClass` _linehitactor "/Game/Blueprints/Components/HoverComponent.HoverComponent_C"))
  (bind _returnvalue_2 (`self.GetComponentByClass` (`self.LineHitActor`) "/Game/Blueprints/Components/HoverComponent.HoverComponent_C"))
  (if (`KismetSystemLibrary.DoesImplementInterface` _linehitactor "/Game/Blueprints/Interfaces/BPI_Magnetic.BPI_Magnetic_C")
    (switch `/Game/Blueprints/Beams/Enum_Magnet_Beam` (`self.Enum_BeamMagnet`)
      (:`NewEnumerator0`
        (`/Game/Blueprints/Components/HoverComponent.StopPull` _returnvalue_2)
        (`/Game/Blueprints/Components/HoverComponent.StopPush` _returnvalue_2))
      (:`NewEnumerator1`
        (`/Game/Blueprints/Components/HoverComponent.Pull` _returnvalue_2 (`SceneComponent.K2_GetComponentLocation` (`self.BeamOutput`)))
        (set `local.Pulled` true))
      (:`NewEnumerator2`
        (`/Game/Blueprints/Components/HoverComponent.Push` (`self.GetComponentByClass` (`self.LineHitActor`) "/Game/Blueprints/Components/HoverComponent.HoverComponent_C") (`self.K2_GetActorRotation` self))
        (set `local.Pushed` true))
      (:`NewEnumerator3`
        (set `/Game/Blueprints/Components/HoverComponent.Floating` (not (`/Game/Blueprints/Components/HoverComponent.Floating` _returnvalue)) _returnvalue)
        (set `self.SignalDone` true)))))

(fn `RightToLeft`
  (locals (LLeftActorLocation :type "Vector Structure" :default (0.0 0.0 0.0)) (LRightActorLocation :type "Vector Structure" :default (0.0 0.0 0.0)) (LOutputLocation :type "Vector Structure" :default (0.0 0.0 0.0)))
  (bind _valid (`self.VerifyLeftRight`))
  (if _valid
    (if (`KismetSystemLibrary.DoesImplementInterface` (`self.LineHitActor`) "/Game/Blueprints/Interfaces/BPI_Magnetic.BPI_Magnetic_C")
      (set `local.LLeftActorLocation` (`self.K2_GetActorLocation` (`self.LeftActor`)))
      (set `local.LRightActorLocation` (`self.K2_GetActorLocation` (`self.RightActor`)))
      (set `local.LOutputLocation` (`self.LineHitLocation`))
      (`self.K2_TeleportTo` :`self` (`self.LeftActor`) :`DestLocation` (`local.LRightActorLocation`))
      (`self.K2_TeleportTo` :`self` (`self.RightActor`) :`DestLocation` (`local.LOutputLocation`))
      (`self.K2_TeleportTo` :`self` (`self.LineHitActor`) :`DestLocation` (`local.LLeftActorLocation`))
      (`self.DestroyBeam`))))

(fn `SignalBeam`
  (bind _linehitactor (`self.LineHitActor`))
  (if (`KismetSystemLibrary.DoesImplementInterface` (`self.LineHitActor`) "/Game/Blueprints/Interfaces/BPI_SignalReceiver.BPI_SignalReceiver_C")
    (switch `/Game/Blueprints/Beams/Enum_SignalBeam` (`self.Enum_BeamSignal`)
      (:`NewEnumerator0`
        (if (`KismetArrayLibrary.Array_Contains` (`Actor.Tags` (`self.LineHitActor`)) "Green")
          (message `/Game/Blueprints/Interfaces/BPI_SignalReceiver.setStatus` _linehitactor true)
          (set `self.SignalDone` true :!label _label)))
      (:`NewEnumerator1`
        (if (`KismetArrayLibrary.Array_Contains` (`Actor.Tags` (`self.LineHitActor`)) "Orange")
          (message `/Game/Blueprints/Interfaces/BPI_SignalReceiver.setStatus` _linehitactor false)
          (goto _label))))))

(fn `UpdateLocationValues`
  (bind _prismbeam (`self.PrismBeam`))
  ;[1 1 1] if a beam exists this will update the source and target location of the beam
  (`/Engine/EditorBlueprintResources/StandardMacros.IsValid` _prismbeam
    (:`Is Valid`
      (set `/Game/Blueprints/Beams/PrismBeams/PrismBeam.SourceLocation` (`SceneComponent.K2_GetComponentLocation` (`self.BeamOutput`)) _prismbeam)
      (set `/Game/Blueprints/Beams/PrismBeams/PrismBeam.TargetLocation` (`self.LineHitLocation`) (`self.PrismBeam`)))))

(fn `UpdateMagnetBeam`
  (params (Enum_Magnet :type "/Game/Blueprints/Beams/Enum_Magnet_Beam Enum" :default "NewEnumerator0"))
  (bind _prismbeam (`self.PrismBeam`))
  (bind _output_get (set `self.Enum_BeamMagnet` Enum_Magnet))
  (`/Engine/EditorBlueprintResources/StandardMacros.IsValid` _prismbeam
    (:`Is Valid`
      (set `/Game/Blueprints/Beams/PrismBeams/PrismBeam.Enum_Magnet` _output_get _prismbeam)
      (set `self.SignalDone` false))))

(fn `UpdateSignalEnum`
  (params (Enum_Signal :type "/Game/Blueprints/Beams/Enum_SignalBeam Enum" :default "NewEnumerator0"))
  (bind _prismbeam (`self.PrismBeam`))
  (if (or (!= Enum_Signal (`self.Enum_BeamSignal`)) (`self.ResetSignalBeam`))
    (bind _output_get (set `self.Enum_BeamSignal` Enum_Signal))
    (`/Engine/EditorBlueprintResources/StandardMacros.IsValid` _prismbeam
      (:`Is Valid`
        (set `/Game/Blueprints/Beams/PrismBeams/PrismBeam.Enum_SignalBeam` _output_get _prismbeam)
        (`/Game/Blueprints/Beams/PrismBeams/PrismBeam.UpdateBeamType` _prismbeam "NewEnumerator0")
        (set `self.SignalDone` false)
        (set `self.ResetSignalBeam` false)))))

(fn `UserConstructionScript`)

(fn `VerifyLeftRight`
  (returns (Valid :type Boolean))
  (`/Engine/EditorBlueprintResources/StandardMacros.IsValid` (`self.LeftActor`)
    (:`Is Valid`
      (`/Engine/EditorBlueprintResources/StandardMacros.IsValid` (`self.RightActor`)
        (:`Is Valid`
          (return true))
        (:`Is Not Valid`
          _)))
    (:`Is Not Valid`
      _))
  (return false))