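; Battery block prop that charges or drains over time and maintains visual beam links to connected actors.
; Tick moves CurrentCharge by rate according to IsCharging, clamped between empty and full, then refreshes materials and beams.
; Two fill meshes show the level through a FillHeight parameter and low, medium or high color bands.
; EstablishConnection spawns one BP_PowerReceptor_Beam per unique target, and DeleteConnection destroys and removes it.
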(event `UpdateConnections`
  (for _array_element (`self.Connections`)
    (`/Game/Blueprints/Props/PowerReceptor/BP_PowerReceptor_Beam.SetTarget` (`.Beam_5_355C101F46A8A56638FC9BA459821808` (break `/Game/Blueprints/Props/Structs/BeamConnection` _array_element)) (break `/Game/Blueprints/Props/Structs/BeamConnection` _array_element))
    (`/Game/Blueprints/Props/PowerReceptor/BP_PowerReceptor_Beam.SetSource` (`.Beam_5_355C101F46A8A56638FC9BA459821808` (break `/Game/Blueprints/Props/Structs/BeamConnection` _array_element)) self)))

(event `self.ReceiveBeginPlay`
  (`self.AdjustMaterial`))

(event `self.ReceiveTick`
  (params (DeltaSeconds :type "Float (single-precision)"))
  (bind _returnvalue (- (`self.currentCharge`) (* (`self.DepleteRatePerSec`) DeltaSeconds)))
  (bind _returnvalue_2 (+ (`self.currentCharge`) (* (`self.ChargeRatePerSec`) DeltaSeconds)))
  (`parent.ReceiveTick` DeltaSeconds)
  (if (`self.isCharging`)
    (if (< _returnvalue_2 100.0)
      (set `self.currentCharge` _returnvalue_2)
      (else
        (set `self.currentCharge` 100.0)))
    (elif (> _returnvalue 0.0)
      (set `self.currentCharge` _returnvalue)
      (else
        (set `self.currentCharge` 0.0))))
  (`self.AdjustMaterial`)
  (`self.UpdateConnections`))

(event `AdjustMaterial`
  (bind _currentcharge (`self.currentCharge`))
  (bind _returnvalue (`KismetMathLibrary.Conv_LinearColorToVector` (`self.chargeColorLow`)))
  (bind _returnvalue_2 (`KismetMathLibrary.Conv_LinearColorToVector` (`self.chargeColorMedium`)))
  (bind _returnvalue_3 (/ (`self.currentCharge`) 100.0))
  (bind _returnvalue_4 (`KismetMathLibrary.Conv_LinearColorToVector` (`self.chargeColorHigh`)))
  (`MeshComponent.SetScalarParameterValueOnMaterials` (`self.Fill`) "FillHeight" _returnvalue_3)
  (`MeshComponent.SetScalarParameterValueOnMaterials` (`self.Fill2`) "FillHeight" _returnvalue_3)
  (if (< _currentcharge 30.0)
    (`MeshComponent.SetVectorParameterValueOnMaterials` (`self.Fill`) "Color" _returnvalue)
    (`MeshComponent.SetVectorParameterValueOnMaterials` (`self.Fill2`) "Color" _returnvalue)
    (elif (< _currentcharge 65.0)
      (`MeshComponent.SetVectorParameterValueOnMaterials` (`self.Fill`) "Color" _returnvalue_2)
      (`MeshComponent.SetVectorParameterValueOnMaterials` (`self.Fill2`) "Color" _returnvalue_2)
      (else
        (`MeshComponent.SetVectorParameterValueOnMaterials` (`self.Fill`) "Color" _returnvalue_4)
        (`MeshComponent.SetVectorParameterValueOnMaterials` (`self.Fill2`) "Color" _returnvalue_4)))))

(event `EstablishConnection`
  (params (BeamTarget :type "Actor Object Reference"))
  (if (== (`KismetArrayLibrary.Array_Length` (`self.Connections`)) 0)
    (bind _returnvalue (`|SpawnActorFromClass` "/Game/Blueprints/Props/PowerReceptor/BP_PowerReceptor_Beam.BP_PowerReceptor_Beam_C" (`self.GetTransform`) "Undefined" "OverrideRootScale" null null :!label _label))
    (`KismetArrayLibrary.Array_Add` (`self.Connections`) (make `/Game/Blueprints/Props/Structs/BeamConnection` BeamTarget _returnvalue))
    (else
      (for _array_element (`self.Connections`)
        (if (== (break `/Game/Blueprints/Props/Structs/BeamConnection` _array_element) BeamTarget)
          (set `self.conExists` true)))
      (if (`self.conExists`)
        (set `self.conExists` false)
        (else
          (goto _label))))))

(event `DeleteConnection`
  (params (`Beam Target` :type "Actor Object Reference"))
  (for (_array_element _array_index) (`self.Connections`)
    (if (== (break `/Game/Blueprints/Props/Structs/BeamConnection` _array_element) `Beam Target`)
      (`self.K2_DestroyActor` (`.Beam_5_355C101F46A8A56638FC9BA459821808` (break `/Game/Blueprints/Props/Structs/BeamConnection` _array_element)))
      (`KismetArrayLibrary.Array_Remove` (`self.Connections`) _array_index))))

(fn `UserConstructionScript`)