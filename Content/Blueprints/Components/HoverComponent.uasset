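; Hover component that floats its owner's first primitive component with physics and lets it be pulled or pushed.
; Each tick while Floating, a downward trace drives a force that weakens with height, using the last ground height on a miss, while a timer alternates trace length to bob it.
; When not floating, physics switches off once vertical velocity reaches zero.
; Pull moves toward a target, Push toward a forward trace hit, both stopping when close.
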(event `self.ReceiveBeginPlay`
  (bind _output_get (set `self.PrimitiveComponent` (`|GetArrayItem` (`Actor.K2_GetComponentsByClass` (`self.GetOwner`) "/Script/Engine.PrimitiveComponent"))))
  (`PrimitiveComponent.SetSimulatePhysics` _output_get (`self.Floating`))
  (`PrimitiveComponent.SetPhysicsMaxAngularVelocityInDegrees` (`self.PrimitiveComponent`) 90.0 false "None")
  (set `self.currentTime` (`self.maxintervaltime`)))

(event `DeactivateComponent`
  (`PrimitiveComponent.SetSimulatePhysics` (`self.PrimitiveComponent`) false))

(event `self.ReceiveTick`
  (params (DeltaSeconds :type "Float (single-precision)"))
  (bind (_returnvalue_x _returnvalue_y) (`KismetMathLibrary.BreakVector` (`self.K2_GetComponentLocation`)))
  (bind _returnvalue (`self.K2_GetComponentLocation`))
  (if (`self.Floating`)
    (`PrimitiveComponent.SetSimulatePhysics` (`self.PrimitiveComponent`) true)
    (bind (_outhit _returnvalue_2) (`KismetSystemLibrary.LineTraceSingle` _returnvalue (- _returnvalue (`KismetMathLibrary.MakeVector` 0.0 0.0 (`self.TraceLength`))) "TraceTypeQuery1"))
    (if _returnvalue_2
      (bind (_bblockinghit _binitialoverlap _time _distance _location _impactpoint _normal _impactnormal) (`GameplayStatics.BreakHitResult` _outhit))
      (set `self.LastHeight` (.z _location))
      (`PrimitiveComponent.AddForce` (`self.PrimitiveComponent`) (* _impactnormal (`KismetMathLibrary.Lerp` (`self.HoverForce`) 0.0 (/ (`KismetMathLibrary.VSize` (- _location (`self.K2_GetComponentLocation`))) (`self.TraceLength`)))) "None" true)
      (else
        (`PrimitiveComponent.AddForce` (`self.PrimitiveComponent`) (* (`KismetMathLibrary.Vector_Up`) (`KismetMathLibrary.Lerp` (`self.HoverForce`) 0.0 (/ (`KismetMathLibrary.VSize` (- (`KismetMathLibrary.MakeVector` _returnvalue_x _returnvalue_y (`self.LastHeight`)) (`self.K2_GetComponentLocation`))) (`self.TraceLength`)))) "None" true)))
    (`PrimitiveComponent.SetLinearDamping` (`self.PrimitiveComponent`) (`self.LinearDamping`))
    (`PrimitiveComponent.SetAngularDamping` (`self.PrimitiveComponent`) (`self.AngularDamping`))
    ;[1 1 1] Added Force Timer
    (if (<= (`self.currentTime`) 0.0)
      (set `self.TraceLength` (+ (`self.TraceLength`) (`self.addedForce`)))
      (set `self.addedForce` (* (`self.addedForce`) -1.0))
      (set `self.currentTime` (`self.maxintervaltime`))
      (else
        (set `self.currentTime` (- (`self.currentTime`) (`GameplayStatics.GetWorldDeltaSeconds`)))))
    (else
      (`KismetSystemLibrary.Delay` 0.1)
      (bind _returnvalue_3 (`PrimitiveComponent.GetPhysicsLinearVelocity` (`self.PrimitiveComponent`) "None"))
      (if (== (.z _returnvalue_3) 0.0)
        (`self.DeactivateComponent`)))))

(event `StopPull`
  (bind _primitivecomponent (`self.PrimitiveComponent`))
  (goto _label :!via `Stop`))

(event `Pull`
  (params (Target :type "Vector Structure"))
  (bind _primitivecomponent (`self.PrimitiveComponent`))
  (bind _returnvalue (`KismetMathLibrary.Vector_Distance` Target (`self.K2_GetComponentLocation` _primitivecomponent)))
  (if (and (`self.Floating`) (>= _returnvalue 100.0))
    (`KismetSystemLibrary.MoveComponentTo` _primitivecomponent Target (struct) false false (/ _returnvalue 120.0) :!label _label)
    (else
      (goto _label :!via `Stop`))))

(event `StopPush`
  (bind _primitivecomponent (`self.PrimitiveComponent`))
  (goto _label_2 :!via `Stop`))

(event `Push`
  (params (Target :type "Rotator Structure"))
  (bind _primitivecomponent (`self.PrimitiveComponent`))
  (bind _returnvalue (`self.K2_GetComponentLocation` _primitivecomponent))
  (bind _outhit (`KismetSystemLibrary.LineTraceSingle` :`Start` _returnvalue :`End` (+ _returnvalue (`KismetMathLibrary.GreaterGreater_VectorRotator` (5000.0 0.0 0.0) Target)) :`TraceChannel` "TraceTypeQuery1" :`DrawDebugType` "ForOneFrame"))
  (if (and (`self.Floating`) (>= (`KismetMathLibrary.Vector_Distance` _returnvalue (`.Location` (`GameplayStatics.BreakHitResult` _outhit))) 150.0))
    (`KismetSystemLibrary.MoveComponentTo` _primitivecomponent (`.Location` (`GameplayStatics.BreakHitResult` _outhit)) (struct) false false (/ (`KismetMathLibrary.Vector_Distance` (`.Location` (`GameplayStatics.BreakHitResult` _outhit)) _returnvalue) 120.0) :!label _label_2)
    (else
      (goto _label_2 :!via `Stop`))))