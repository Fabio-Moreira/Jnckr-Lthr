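; BP_BBShowOff is a decorative prop for the main menu that displays a random charge level.
; On BeginPlay it picks a random CurrentCharge and a random rotation, roll included.
; AdjustMaterial writes the normalized charge to the FillHeight material parameter on both Fill components and tints them with a low, medium or high color by threshold.
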(event `self.ReceiveBeginPlay`
  (set `self.currentCharge` (`KismetMathLibrary.RandomFloatInRange` 0.0 100.0))
  (`self.AdjustMaterial`)
  (`self.K2_SetActorRotation` (`KismetMathLibrary.RandomRotator` true)))

(event `AdjustMaterial`
  (bind _fill1 (`self.Fill1`))
  (bind _currentcharge (`self.currentCharge`))
  (bind _returnvalue (`KismetMathLibrary.Conv_LinearColorToVector` (`self.chargeColorLow`)))
  (bind _returnvalue_2 (`KismetMathLibrary.Conv_LinearColorToVector` (`self.chargeColorMedium`)))
  (bind _returnvalue_3 (/ (`self.currentCharge`) 100.0))
  (bind _returnvalue_4 (`KismetMathLibrary.Conv_LinearColorToVector` (`self.chargeColorHigh`)))
  (`MeshComponent.SetScalarParameterValueOnMaterials` (`self.Fill`) "FillHeight" _returnvalue_3)
  (`MeshComponent.SetScalarParameterValueOnMaterials` (`self.Fill1`) "FillHeight" _returnvalue_3)
  (if (< _currentcharge 30.0)
    (`MeshComponent.SetVectorParameterValueOnMaterials` (`self.Fill`) "Color" _returnvalue)
    (`MeshComponent.SetVectorParameterValueOnMaterials` (`self.Fill1`) "Color" _returnvalue)
    (elif (< _currentcharge 65.0)
      (`MeshComponent.SetVectorParameterValueOnMaterials` (`self.Fill`) "Color" _returnvalue_2)
      (`MeshComponent.SetVectorParameterValueOnMaterials` _fill1 "Color" _returnvalue_2)
      (else
        (`MeshComponent.SetVectorParameterValueOnMaterials` (`self.Fill`) "Color" _returnvalue_4)
        (`MeshComponent.SetVectorParameterValueOnMaterials` _fill1 "Color" _returnvalue_4)))))

(fn `UserConstructionScript`)